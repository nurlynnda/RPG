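; Melee combat component for the third-person character, running a four-step sword and kick combo from the attack input.
; Presses during an attack are buffered in SaveAttack, and SwordAttackCombo either plays the next montage by AttackIndex or resets the combo.
; A looping timer sphere-traces between the sword's end points, throttled by a DoOnce, while SphereTrace does a single point check.
; Both traces damage "Damageable"-tagged actors and spawn blood effects.
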(event `self.ReceiveBeginPlay`
  (bind _asbp_third_person_character (cast `/Game/ThirdPerson/Blueprints/BP_ThirdPersonCharacter` (`self.GetOwner`)))
  (set `self.Character BP` _asbp_third_person_character)
  (set `self.CharacterMesh` (`Character.Mesh` _asbp_third_person_character)))

(event `EnhancedInput|/Game/ThirdPerson/Input/Actions/IA_Attack`
  (params (ActionValue :type Boolean) (ElapsedSeconds :type "Float (double-precision)") (TriggeredSeconds :type "Float (double-precision)") (InputAction :type "InputAction Object Reference" :default "/Game/ThirdPerson/Input/Actions/IA_Attack.IA_Attack"))
  ; combo system
  ;; AttackInput
  (:`Started`
    (if (`self.canAttack`)
      (`self.SwordAttack`))))

(event `Attack1`
  ; combo system
  ;; Attack 1
  (`/Engine/EditorBlueprintResources/StandardMacros.DoOnce` false :!label _label
    (:`Completed`
      (`KismetSystemLibrary.Delay` 0.1)
      (`|PlayMontage` (`self.CharacterMesh`) "/Game/Characters/RPG_Character/Annimation/SwordAttack/Attack1_Montage.Attack1_Montage"
        (:`then`
          (set `self.Attack Index` 1)
          (goto _label :!via `Reset`))))))

(event `SwordAttack`
  ; combo system
  ;; SwordAttack
  (if (`self.isAttacking`)
    (set `self.saveAttack` true)
    (else
      (set `self.isAttacking` true)
      (switch `int` (`self.Attack Index`) :!label _label_2
        (:`0`
          (`self.Attack1`))
        (:`1`
          (`self.Attack 2`))
        (:`2`
          (`self.Attack 3`))
        (:`3`
          (`self.Kick`))))))

(event `Attack 2`
  ; combo system
  ;; Attack 2
  (`/Engine/EditorBlueprintResources/StandardMacros.DoOnce` false :!label _label_3
    (:`Completed`
      (`KismetSystemLibrary.Delay` 0.1)
      (`|PlayMontage` (`self.CharacterMesh`) "/Game/Characters/RPG_Character/Annimation/SwordAttack/Attack2_Montage.Attack2_Montage"
        (:`then`
          (set `self.Attack Index` 2)
          (goto _label_3 :!via `Reset`))))))

(event `SwordAttackCombo`
  ; combo system
  ;; Combo Continue
  (if (`self.saveAttack`)
    (set `self.saveAttack` false)
    (goto _label_2)
    (else
      (`self.StopCombo`))))

(event `Attack 3`
  ; combo system
  ;; Attack 3
  (`/Engine/EditorBlueprintResources/StandardMacros.DoOnce` false :!label _label_4
    (:`Completed`
      (`KismetSystemLibrary.Delay` 0.1)
      (`|PlayMontage` (`self.CharacterMesh`) "/Game/Characters/RPG_Character/Annimation/SwordAttack/Kick_Montage.Kick_Montage"
        (:`then`
          (set `self.Attack Index` 3)
          (goto _label_4 :!via `Reset`))))))

(event `StopCombo`
  ; combo system
  ;; Stop Combo/Attack
  (set `self.isAttacking` false)
  (set `self.Attack Index` 0))

(event `Kick`
  ; combo system
  ;; Kick
  (`/Engine/EditorBlueprintResources/StandardMacros.DoOnce` false :!label _label_5
    (:`Completed`
      (`KismetSystemLibrary.Delay` 0.1)
      (`|PlayMontage` (`self.CharacterMesh`) "/Game/Characters/RPG_Character/Annimation/SwordAttack/Attack3_Montage.Attack3_Montage"
        (:`then`
          (set `self.Attack Index` 4)
          (goto _label_5 :!via `Reset`))))))

(event `Start Sword Trace`
  ; sword trace
  (bind _returnvalue (`KismetSystemLibrary.K2_SetTimerDelegate` (delegate `Sword Trace Loop`) 0.01 true))
  (set `self.SwordTraceLoop` _returnvalue))

(event `SphereTrace`
  (bind _returnvalue (`SceneComponent.K2_GetComponentLocation` (`/Game/ThirdPerson/Blueprints/BP_ThirdPersonCharacter.SphereTrace` (`self.Character BP`))))
  ; Sphere Trace
  (bind (_outhit _returnvalue_2) (`KismetSystemLibrary.SphereTraceSingle` _returnvalue _returnvalue 0.0 "TraceTypeQuery1"))
  (if _returnvalue_2
    (bind (_bblockinghit _binitialoverlap _time _distance _location _impactpoint _normal _impactnormal _physmat _hitactor) (`GameplayStatics.BreakHitResult` _outhit))
    (if (`Actor.ActorHasTag` _hitactor "Damageable")
      (`GameplayStatics.ApplyDamage` _hitactor 10.0)
      (`GameplayStatics.SpawnEmitterAtLocation` "/Game/FX/Particles/Blood/P_Blood_Splat_Cone.P_Blood_Splat_Cone" _location (`KismetMathLibrary.MakeRotFromXY` _normal _normal) (0.4 0.4 0.4) true "AutoRelease"))))

(event `Sword Trace Loop`
  ; sword trace
  (bind (_outhit _returnvalue) (`KismetSystemLibrary.SphereTraceSingle` :`Start` (`SceneComponent.K2_GetComponentLocation` (`/Game/ThirdPerson/Blueprints/BP_ThirdPersonCharacter.Sword Top Point` (`self.Character BP`))) :`End` (`SceneComponent.K2_GetComponentLocation` (`/Game/ThirdPerson/Blueprints/BP_ThirdPersonCharacter.Sword Bottom Point` (`self.Character BP`))) :`Radius` 12.0 :`TraceChannel` "TraceTypeQuery1" :`DrawTime` 0.2))
  (if _returnvalue
    (bind (_bblockinghit _binitialoverlap _time _distance _location _impactpoint _normal _impactnormal _physmat _hitactor) (`GameplayStatics.BreakHitResult` _outhit))
    (if (`Actor.ActorHasTag` _hitactor "Damageable")
      (`/Engine/EditorBlueprintResources/StandardMacros.DoOnce` false :!label _label_6
        (:`Completed`
          (`GameplayStatics.ApplyDamage` _hitactor 10.0)
          (`GameplayStatics.SpawnEmitterAtLocation` "/Game/FX/Particles/Blood/P_Blood_Splat_Cone.P_Blood_Splat_Cone" _location (`KismetMathLibrary.MakeRotFromXY` _normal _normal) (0.4 0.4 0.4) true "AutoRelease")
          (`KismetSystemLibrary.Delay` 0.5)
          (goto _label_6 :!via `Reset`))))))

(event `StopSwordTrace`
  ; sword trace
  (`KismetSystemLibrary.K2_ClearAndInvalidateTimerHandle` (`self.SwordTraceLoop`)))